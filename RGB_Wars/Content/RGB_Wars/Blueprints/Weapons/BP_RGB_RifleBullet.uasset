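; BP_RGB_RifleBullet is the RGB Wars rifle projectile that handles impact effects and sounds when it hits something.
; Its hit event spawns a full explosion actor when the bullet is destroyed, adding a despawn sound only if no damage was dealt.
; Hits that leave the bullet alive spawn a small explosion and play a bounce sound.
; The construction script only calls its parent.
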(event EventOnProjectileHit
  (params (Hit :type Hit%20Result%20Structure%20%28by%20ref%29) (GetsDestroyed :type Boolean) (DidDamage :type Boolean))
  (bind _returnvalue (Transformation|GetActorTransform))
  (if GetsDestroyed
    (if DidDamage
      (Game|SpawnActorfromClass "/Game/RGB_Wars/Blueprints/Weapons/BP_RGB_Bullet_Explosion.BP_RGB_Bullet_Explosion_C" _returnvalue "AlwaysSpawn" "MultiplyWithRoot" 0 0)
      (else
        (bind _returnvalue_2 (Game|SpawnActorfromClass "/Game/RGB_Wars/Blueprints/Weapons/BP_RGB_Bullet_Explosion.BP_RGB_Bullet_Explosion_C" _returnvalue "AlwaysSpawn" "MultiplyWithRoot" 0 0))
        (Audio|PlaySoundatLocation "/Game/RGB_Wars/Sound/Bullet/S_RGB_Bullet_Despawn.S_RGB_Bullet_Despawn" (Transformation|GetActorLocation _returnvalue_2) "0, 0, 0" 1.0 1.0 0.0 0 0 0 0)))
    (else
      (bind _returnvalue_3 (Game|SpawnActorfromClass "/Game/RGB_Wars/Blueprints/Weapons/BP_RGB_Bullet_Explosion_Small.BP_RGB_Bullet_Explosion_Small_C" _returnvalue "AlwaysSpawn" "MultiplyWithRoot" 0 0))
      (Audio|PlaySoundatLocation "/Game/RGB_Wars/Sound/Bullet/S_RGB_Bullet_Bounce.S_RGB_Bullet_Bounce" (Transformation|GetActorLocation _returnvalue_3) "0, 0, 0" 1.0 1.0 0.0 0 0 0 0))))

(fn ConstructionScript
  (|CallParentFunction))