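; BP_RGB_Bullet_Explosion is a short-lived bullet explosion effect in RGB Wars, shown as a sphere colored to the shooter.
; On BeginPlay it sets the sphere's material from the instigating BP_RGB_Character's RGB color, falling back to white when the instigator is invalid, such as a dead player.
; A timeline then scales the sphere by a size curve times a multiplier and destroys the actor when finished.
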(event EventBeginPlay
  (bind _returnvalue (Game|GetInstigator))
  (Utilities|FlowControl|Sequence
    (:then_0
      (if (Utilities|IsValid _returnvalue)
        (bind _asbp_rgb_character (Utilities|Casting|CastToBP_RGB_Character _returnvalue))
        (bind _material (CallFunction|GetExplosionMaterialbyRGB (Variables|/Game/RGB_Wars/Blueprints/Characters/BP_RGB_Character.BP_RGB_Character_C|GetRGBColor _asbp_rgb_character)))
        (Rendering|Material|SetMaterial (Variables|Default|GetSphere) 0 _material)
        (else
          ;[0.15 0.15 0.15 0.5] If Player is dead then make bullet explosions White (would have Error otherwise)
          (bind _material_2 (CallFunction|GetExplosionMaterialbyRGB "NewEnumerator3"))
          (Rendering|Material|SetMaterial (Variables|Default|GetSphere) 0 _material_2))))
    (:then_1
      (bind _size (Timeline|Timeline PlayFromStart)
        (:Update
          (Transformation|SetRelativeScale3D (Variables|Default|GetSphere) (Math|Conversions|ToVector(Float) (* _size (Variables|Default|GetExplosionSizeMult)))))
        (:Finished
          (Actor|DestroyActor))))))

(fn ConstructionScript)