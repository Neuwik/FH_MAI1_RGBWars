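; Player controller for RGB Wars that sets up input and handles players joining and pausing.
; BeginPlay caches the shooter game mode, then adds the default and separate mouse-look Enhanced Input contexts after a short delay.
; Join input, gated by a 255 PlayerIndex as the unregistered sentinel, registers with the game mode, saves the index and restarts at a random spawn.
; Pause input asks the game mode to toggle the settings UI.
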(event Input|EnhancedActionEvents|EnhancedInputActionIA_JoinGame
  (params (ActionValue :type Boolean) (ElapsedSeconds :type Float%20%28double-precision%29) (TriggeredSeconds :type Float%20%28double-precision%29) (InputAction :type Input%20Action%20Object%20Reference :default "/Game/Input/Actions/IA_JoinGame.IA_JoinGame"))
  (bind _self self)
  (bind _gm_as_gm_rgb_shooter (Variables|Default|GetGM_as_GM_RGB_Shooter))
  (if ActionValue
    (Math|Integer|CompareInt (Math|Conversions|ToInteger(Byte) (Variables|Default|GetPlayerIndex)) 255
      (:==
        (CallFunction|RegisterPlayerandSaveIndex _self)
        (bind _spawn (Default|GetNextRandomSpawnPoint _gm_as_gm_rgb_shooter))
        (Class|GameModeBase|RestartPlayeratPlayerStart _gm_as_gm_rgb_shooter _self _spawn)))))

(event Input|EnhancedActionEvents|EnhancedInputActionIA_Pause
  (params (ActionValue :type Boolean) (ElapsedSeconds :type Float%20%28double-precision%29) (TriggeredSeconds :type Float%20%28double-precision%29) (InputAction :type Input%20Action%20Object%20Reference :default "/Game/Input/Actions/IA_Pause.IA_Pause"))
  (if ActionValue
    (Default|ToggleSettingsUI (Variables|Default|GetGM_as_GM_RGB_Shooter))))

(event EventBeginPlay
  (bind _self self)
  (bind _returnvalue (PlayerController|LocalPlayerSubsystems|GetEnhancedInputLocalPlayerSubsystem _self))
  ;[0.15 0.15 0.15 0.5] Initialize player input
  (bind _asgm_rgb_shooter (Utilities|Casting|CastToGM_RGB_Shooter (Game|GetGameMode)))
  (Variables|Default|SetGM_as_GM_RGB_Shooter _asgm_rgb_shooter)
  (Utilities|FlowControl|Delay 0.2)
  (Utilities|IsValid _returnvalue
    (:Is%20Valid
      (Utilities|FlowControl|Sequence
        (:then_0
          ;;[0.15 0.15 0.15 0.5] Add regular input mappings
          (Input|AddMappingContext _returnvalue "/Game/Input/IMC_Default.IMC_Default" 0 "(bIgnoreAllPressedKeysUntilRelease=True,bForceImmediately=False,bNotifyUserSettings=False)"))
        (:then_1
          ;;[0.15 0.15 0.15 0.5] Add MouseLook input mappings (Seperate because of template mobile controls)
          (Input|AddMappingContext _returnvalue "/Game/Input/IMC_MouseLook.IMC_MouseLook" 0 "(bIgnoreAllPressedKeysUntilRelease=True,bForceImmediately=False,bNotifyUserSettings=False)"))))))

(fn ConstructionScript)

(fn RegisterPlayerandSaveIndex
  (bind _playerrgbcolor (Default|RegisterPlayer (Variables|Default|GetGM_as_GM_RGB_Shooter) self))
  (Variables|Default|SetPlayerIndex _playerrgbcolor))