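; Game mode for RGB Wars, a local multiplayer shooter that runs the lobby, timed match, win screen and restart.
; It creates local players, assigns colors on registration and swaps widgets, pausing the game outside matches.
; Per-player HP and score maps broadcast changes through dispatchers, with kills and damage earning points and the top score or a draw declared.
; Spawns draw randomly from a refilling index pool, avoiding repeats until exhausted.
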(event Custom|StopMatch
  (Variables|Default|SetMatchRunning false)
  (Game|SetGamePaused true)
  (bind _playerrgbcolor (CallFunction|GetLeadingPlayer))
  (CallFunction|SetUIActive (Variables|UI|GetWinUI))
  (Default|CallWinnerDelcared _playerrgbcolor))

(event Custom|StartMatch
  (bind _matchui (Variables|UI|GetMatchUI))
  (CallFunction|SetUIActive _matchui)
  (CallFunction|ResetPlayerScores)
  (bind (_minutes _seconds) (CallFunction|SecondstoMinutesandSeconds (Variables|Default|GetMatchDuration)))
  (Default|ResetTimer _matchui _minutes _seconds true)
  (EventDispatchers|BindEventtoTimerFinished _matchui (delegate Custom|TimerFinishedCallback))
  (Game|SetGamePaused false)
  (Variables|Default|SetMatchRunning true))

(event Custom|RestartMatch
  (Utilities|Array|Clear (Variables|PlayerRespawning|GetAvailableSpawnIndexes))
  (bind _outactors (Actor|GetAllActorsOfClass "/Game/RGB_Wars/Blueprints/Weapons/BP_RGB_ProjectileBase.BP_RGB_ProjectileBase_C"))
  (for _array_element _outactors
    (Actor|DestroyActor _array_element))
  (bind _outactors_2 (Actor|GetAllActorsOfClass (Variables|Default|GetDefaultPawnClass)))
  (for _array_element_2 _outactors_2
    (CallFunction|RespawnPlayer (Pawn|GetController _array_element_2)))
  (CallFunction|SetUIActive (Variables|UI|GetLobbyUI))
  (Default|CallAllPlayersReady))

(event Custom|TimerFinishedCallback
  (CallFunction|StopMatch))

(event Custom|RespawnPlayer
  (params (PlayerController :type Controller%20Object%20Reference))
  (bind _returnvalue (Pawn|GetControlledPawn PlayerController))
  (Utilities|IsValid _returnvalue
    (:Is%20Valid
      (Actor|DestroyActor _returnvalue))
    (:Is%20Not%20Valid
      _))
  (CallFunction|SpawnPlayer PlayerController))

(event Custom|SpawnPlayer
  (params (PlayerController :type Controller%20Object%20Reference))
  (bind _spawn (CallFunction|GetNextRandomSpawnPoint))
  (Class|GameModeBase|RestartPlayeratPlayerStart PlayerController _spawn))

(event Custom|ToggleSettingsUI
  (Default|ToggleSettings (Variables|UI|GetSettingsUI) (Variables|UI|GetFocusedWidget))
  (if (Variables|Default|GetMatchRunning)
    (Game|SetGamePaused (not (Game|IsGamePaused)))))

(event Custom|OnAllPlayersJoined
  (Default|CallAllPlayersReady))

(event Custom|ExitGame
  (Utilities|FlowControl|Delay 0.1)
  (Game|QuitGame (Game|GetPlayerController 0) "Quit" false))

(event EventBeginPlay
  (bind _outactors (Actor|GetAllActorsOfClass "/Script/Engine.PlayerStart"))
  (Variables|PlayerRespawning|SetSpawnPoints _outactors)
  (for _index (range 0 (- (Variables|Default|GetMaxPlayerCount) 2))
    (Class|GameplayStatics|CreatePlayer -1))
  (Utilities|FlowControl|Sequence
    (:then_0
      (Variables|Default|SetDefaultPawnClass "/Game/RGB_Wars/Blueprints/Characters/BP_RGB_ShooterCharacter.BP_RGB_ShooterCharacter_C"))
    (:then_1
      (CallFunction|CreateUI)
      (CallFunction|SetUIActive (Variables|UI|GetLobbyUI)))
    (:then_2
      (Utilities|FlowControl|Sequence
        (:then_0
          (EventDispatchers|BindEventtoAllPlayersJoined (delegate Custom|OnAllPlayersJoined)))
        (:then_1
          (EventDispatchers|BindEventtoCountdownFinished (Variables|UI|GetLobbyUI) (delegate Custom|StartMatch)))
        (:then_2
          (EventDispatchers|BindEventtoResumeButtonPressed (Variables|UI|GetSettingsUI) (delegate Custom|ToggleSettingsUI)))))
    (:then_3
      (Audio|PushSoundMixModifier (Variables|Default|GetSoundMixModifier))
      (Audio|PlaySound2D "/Game/RGB_Wars/Sound/Music/S_RGB_BackgroundMusic.S_RGB_BackgroundMusic" 1.0 1.0 0.0 0 0))
    (:then_4
      ;[0.15 0.15 0.15 0.5] Delay to let Camera and PCs Spawn and then Pause the game.
      (Utilities|FlowControl|Delay 0.2)
      (Game|SetGamePaused true))))

(event EventIncreasePlayerScorebyDmg
  (params (PlayerIndex :type Byte :default 0) (Damage :type Integer))
  (CallFunction|IncreasePlayerScore PlayerIndex (Math|Float|Round (* Damage (Variables|PlayerScores|GetDamageScoreModifier)))))

(event EventIncreasePlayerScorebyKill
  (params (PlayerIndex :type Byte :default 0))
  (CallFunction|IncreasePlayerScore PlayerIndex (Math|Float|Truncate (Variables|PlayerScores|GetKillScoreModifier))))

(event EventResetPlayerScores
  (bind _playerscores (Variables|PlayerScores|GetPlayerScores))
  (bind _keys (Utilities|Map|Keys _playerscores))
  (for _array_element _keys
    (Utilities|Map|Add _playerscores _array_element 0))
  (Default|CallPlayerScoresUpdated (Variables|PlayerScores|GetPlayerScores)))

(fn ConstructionScript)

(fn IncreaseJoinedPlayerCount
  (bind _maxplayercount (Variables|Default|GetMaxPlayerCount))
  (Variables|Default|SetJoinedPlayerCount (+ (Variables|Default|GetJoinedPlayerCount) 1))
  (Default|CallJoinedPlayersUpdated (Variables|Default|GetJoinedPlayerCount) _maxplayercount)
  (if (>= (Variables|Default|GetJoinedPlayerCount) _maxplayercount)
    (Default|CallAllPlayersJoined)))

(fn ResetPlayerHP
  (params (PlayerIndex :type Byte))
  (bind _playermaxhp (Variables|PlayerHP|GetPlayerMaxHP))
  (Utilities|Map|Add (Variables|PlayerHP|GetPlayerHPs) PlayerIndex _playermaxhp)
  (Default|CallPlayerHPsUpdated (Variables|PlayerHP|GetPlayerHPs))
  (return _playermaxhp 1.0 true))

(fn SetPlayerHP
  (params (PlayerIndex :type Byte) (Amount :type Integer))
  (bind _playermaxhp (Variables|PlayerHP|GetPlayerMaxHP))
  (bind _playerhps (Variables|PlayerHP|GetPlayerHPs))
  (Math|Integer|CompareInt Amount _playermaxhp
    (:>
      _)
    (:==
      _)
    (:<
      (Math|Integer|CompareInt Amount
        (:>
          (Utilities|Map|Add _playerhps PlayerIndex Amount)
          (Default|CallPlayerHPsUpdated (Variables|PlayerHP|GetPlayerHPs))
          (return Amount (Math|Float|SafeDivide (Math|Conversions|ToFloat(Integer) Amount) (Math|Conversions|ToFloat(Integer) _playermaxhp)) true))
        (:==
          _)
        (:<
          _))
      (Utilities|Map|Add _playerhps PlayerIndex 0)
      (Default|CallPlayerHPsUpdated (Variables|PlayerHP|GetPlayerHPs))
      (return 0 0.0 false)))
  (Utilities|Map|Add _playerhps PlayerIndex _playermaxhp)
  (Default|CallPlayerHPsUpdated (Variables|PlayerHP|GetPlayerHPs))
  (return _playermaxhp 1.0 true))

(fn IncreasePlayerHP
  (params (PlayerIndex :type Byte) (Amount :type Integer))
  (bind _output_get (LocalVariables|SetPrevHP (.Value (Utilities|Map|Find (Variables|PlayerHP|GetPlayerHPs) PlayerIndex))))
  (bind (_newhp _newpercenthp _isalive) (CallFunction|SetPlayerHP PlayerIndex (+ _output_get Amount)))
  (return _newhp _newpercenthp _isalive (- _newhp _output_get)))

(fn DecreasePlayerHP
  (params (PlayerIndex :type Byte) (Amount :type Integer))
  (bind _output_get (LocalVariables|SetPrevHÜ (.Value (Utilities|Map|Find (Variables|PlayerHP|GetPlayerHPs) PlayerIndex))))
  (bind (_newhp _newpercenthp _isalive) (CallFunction|SetPlayerHP PlayerIndex (- _output_get Amount)))
  (return _newhp _newpercenthp _isalive (- _output_get _newhp)))

(fn IncreasePlayerScore
  (params (PlayerIndex :type Byte) (Amount :type Integer))
  (bind _playerscores (Variables|PlayerScores|GetPlayerScores))
  (Utilities|Map|Add _playerscores PlayerIndex (+ (.Value (Utilities|Map|Find _playerscores PlayerIndex)) Amount))
  (Default|CallPlayerScoresUpdated (Variables|PlayerScores|GetPlayerScores)))

(fn GetNextRandomSpawnPoint
  (bind _availablespawnindexes (Variables|PlayerRespawning|GetAvailableSpawnIndexes))
  (bind _spawnpoints (Variables|PlayerRespawning|GetSpawnPoints))
  (if (Utilities|Array|IsNotEmpty _spawnpoints)
    (if (Utilities|Array|IsNotEmpty (Variables|PlayerRespawning|GetAvailableSpawnIndexes))
      ;[0.15 0.15 0.15 0.5] Get Random Spawn
      (LocalVariables|SetIndexOfSpawnIndex (.OutIndex (Utilities|Array|Random (Variables|PlayerRespawning|GetAvailableSpawnIndexes))) :!label _label)
      (bind _output_get (LocalVariables|SetSpawnIndex (Utilities|Array|Get(acopy) _availablespawnindexes (LocalVariables|GetIndexOfSpawnIndex))))
      (Utilities|Array|RemoveIndex _availablespawnindexes (LocalVariables|GetIndexOfSpawnIndex))
      (return (Utilities|Array|Get(acopy) (Variables|PlayerRespawning|GetSpawnPoints) _output_get))
      (else
        (Utilities|FlowControl|Sequence
          (:then_0
            ;[0.15 0.15 0.15 0.5] Repopulate Available Spawn Indexes
            (for _index (range 0 (- (Utilities|Array|Length _spawnpoints) 1))
              (Utilities|Array|Add (Variables|PlayerRespawning|GetAvailableSpawnIndexes) _index)))
          (:then_1
            (goto _label)))))))

(fn GetLeadingPlayer
  (bind (_keypin _valuepin) (Utilities|Map|ForEachLoop(Map) (Variables|PlayerScores|GetPlayerScores))
    (:then
      (if (> _valuepin (LocalVariables|GetCurrentScoresPoints))
        (LocalVariables|SetCurrentLeaderIndex _keypin)
        (LocalVariables|SetCurrentScoresPoints _valuepin)
        (LocalVariables|SetIsDraw false)
        (else
          (LocalVariables|SetIsDraw (== _valuepin (LocalVariables|GetCurrentScoresPoints))))))
    (:CompletedPin
      (if (LocalVariables|GetIsDraw)
        (return "NewEnumerator3")
        (else
          (return (Utilities|Enum|ByteToEnumE_RGB_Colors (LocalVariables|GetCurrentLeaderIndex))))))))

(fn CreateUI
  (Utilities|FlowControl|Sequence
    (:then_0
      (bind _returnvalue (UserInterface|CreateWidget "/Game/RGB_Wars/UI/UI_RGB_Lobby.UI_RGB_Lobby_C"))
      (Variables|UI|SetLobbyUI _returnvalue))
    (:then_1
      (bind _returnvalue_2 (UserInterface|CreateWidget "/Game/RGB_Wars/UI/UI_RGB_Match.UI_RGB_Match_C"))
      (Variables|UI|SetMatchUI _returnvalue_2))
    (:then_2
      (bind _returnvalue_3 (UserInterface|CreateWidget "/Game/RGB_Wars/UI/UI_RGB_Win.UI_RGB_Win_C"))
      (Variables|UI|SetWinUI _returnvalue_3))
    (:then_3
      (bind _returnvalue_4 (UserInterface|CreateWidget "/Game/RGB_Wars/UI/UI_RGB_Settings.UI_RGB_Settings_C"))
      (bind _output_get (Variables|UI|SetSettingsUI _returnvalue_4))
      (UserInterface|Viewport|AddtoViewport _output_get 10))))

(fn SetUIActive
  (params (UI :type User%20Widget%20Object%20Reference) (OwningPlayer :type Player%20Controller%20Object%20Reference))
  (UserInterface|Viewport|AddtoViewport UI 0)
  (if (Variables|/Script/UMG.UserWidget|GetbIsFocusable UI)
    (Variables|UI|SetFocusedWidget UI)))

(fn RegisterPlayer
  (params (Player%20Controller :type PC%20RGB%20Player%20Controller%20Object%20Reference))
  (bind _output_get (LocalVariables|SetRGBColor (Utilities|Enum|ByteToEnumE_RGB_Colors (Math|Conversions|ToByte(Integer) (Variables|Default|GetJoinedPlayerCount)))))
  (Utilities|Map|Add (Variables|Default|GetPlayerControllersByRGBColors) _output_get Player%20Controller)
  (CallFunction|IncreaseJoinedPlayerCount)
  (return _output_get))